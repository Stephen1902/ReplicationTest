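; Campfire world item that toggles its fire particle system on or off when its WarmingSphere is hit.
; A hit prints a debug message, then toggles directly with authority or calls ServerParticle on remote machines.
; The projectile class check gates nothing as both branches are empty.
; The toggle also sets IsActive, whose OnRep function is empty.
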(event `self.ReceiveBeginPlay`)

(event `ServerParticle`
  (bind _particlesystem (`self.ParticleSystem`))
  (if (== (`GameplayStatics.GetObjectClass` (stale `self.WarmingSphere.OnComponentHit` OtherActor)) "/Game/FirstPersonCPP/Blueprints/FirstPersonProjectile.FirstPersonProjectile_C") :!label _label
    _
    (else
      _))
  (if (`ActorComponent.IsActive` _particlesystem)
    (`ActorComponent.Deactivate` _particlesystem)
    (set `self.IsActive` false)
    (else
      (`ActorComponent.Activate` _particlesystem false)
      (set `self.IsActive` true))))

(event `self.WarmingSphere.OnComponentHit`
  (params (HitComponent :type "PrimitiveComponent Object Reference") (OtherActor :type "Actor Object Reference") (OtherComp :type "PrimitiveComponent Object Reference") (NormalImpulse :type "Vector Structure") (Hit :type "HitResult Structure (by ref)"))
  (`KismetSystemLibrary.PrintString` "Ouch!")
  (`/Engine/EditorBlueprintResources/ActorMacros.Switch Has Authority`
    (:`Authority`
      (goto _label))
    (:`Remote`
      (`self.ServerParticle`))))

(fn `OnRep_IsActive`)

(fn `UserConstructionScript`)